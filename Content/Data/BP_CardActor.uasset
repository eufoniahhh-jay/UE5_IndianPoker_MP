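; Card actor that displays a card's face and back on its mesh through a dynamic instance of M_Card.
; BeginPlay creates the material instance with the default back, and SetCardTextures recreates it if invalid.
; UpdateCardVisual maps a positive 1-based value to a front texture, swapping in a per-value back when revealed.
; SetCardFrontOnly sets a given front with the default back, while OnCardValueChanged is an empty stub.
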(event EventBeginPlay
  (CallFunction|InitializeCardMaterial))

(event Collision|EventActorBeginOverlap
  (params (OtherActor :type Actor%20Object%20Reference)))

(event EventTick
  (params (DeltaSeconds :type Float%20%28single-precision%29)))

(event EventSetCardFrontOnly
  (params (InFrontTexture :type Texture%202D%20Object%20Reference))
  (CallFunction|SetCardFrontOnly InFrontTexture))

(event EventOnCardValueChanged
  (params (InCardValue :type Integer)))

(event EventUpdateCardVisual
  (params (InCardValue :type Integer) (bInRevealed :type Boolean))
  (bind _returnvalue (- InCardValue 1))
  (if (> InCardValue 0)
    (if bInRevealed
      (CallFunction|SetCardTextures (Utilities|Array|Get(acopy) (Variables|Default|GetFrontTextures) _returnvalue) (Utilities|Array|Get(acopy) (Variables|Default|GetRevealBackTextures) _returnvalue))
      (else
        (CallFunction|SetCardTextures (Utilities|Array|Get(acopy) (Variables|Default|GetFrontTextures) (- InCardValue 1)) (Variables|Default|GetBackTexture))))))

(fn ConstructionScript)

(fn InitializeCardMaterial
  (bind _returnvalue (Rendering|Material|CreateDynamicMaterialInstance (Variables|Default|GetCardMesh) 0 "/Game/Data/CardsImage/M_Card.M_Card" "None" :!class /Script/Engine.PrimitiveComponent))
  (bind _output_get (Variables|Default|SetCardMID _returnvalue))
  (Utilities|IsValid _output_get
    (:Is%20Valid
      (Rendering|Material|SetTextureParameterValue _output_get "BackTexture" (Variables|Default|GetBackTexture)))))

(fn SetCardTextures
  (params (InFrontTexture :type Texture%202D%20Object%20Reference) (InBackTexture :type Texture%202D%20Object%20Reference))
  (bind _cardmid (Variables|Default|GetCardMID))
  (bind _cardmid_2 (Variables|Default|GetCardMID))
  (if (Utilities|IsValid (Variables|Default|GetCardMID))
    (Rendering|Material|SetTextureParameterValue _cardmid_2 "FrontTexture" InFrontTexture)
    (Rendering|Material|SetTextureParameterValue _cardmid_2 "BackTexture" InBackTexture)
    (else
      (CallFunction|InitializeCardMaterial)
      (Rendering|Material|SetTextureParameterValue _cardmid "FrontTexture" InFrontTexture)
      (Rendering|Material|SetTextureParameterValue _cardmid "BackTexture" InBackTexture))))

(fn SetCardFrontOnly
  (params (InFrontTexture :type Texture%202D%20Object%20Reference))
  (bind _cardmid (Variables|Default|GetCardMID))
  (Rendering|Material|SetTextureParameterValue _cardmid "FrontTexture" InFrontTexture)
  (Rendering|Material|SetTextureParameterValue _cardmid "BackTexture" (Variables|Default|GetBackTexture)))