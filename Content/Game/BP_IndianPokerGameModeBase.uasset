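; BP_IndianPokerGameModeBase is the game mode for an Indian Poker game, giving the local player's character a card on start.
; Shortly after BeginPlay, it casts the first player controller's pawn to BP_IPCharacter and spawns a BP_CardActor just above it.
; The card snaps to the character's CardAnchor component, keeping its world scale.
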(event EventBeginPlay
  (Utilities|FlowControl|Delay 0.2)
  (bind _asbp_ipcharacter (Utilities|Casting|CastToBP_IPCharacter (Pawn|GetControlledPawn (Game|GetPlayerController 0))))
  (bind _returnvalue (Game|SpawnActorfromClass "/Game/Data/BP_CardActor.BP_CardActor_C" (Math|Conversions|ToTransform(Vector) (+ (Transformation|GetActorLocation _asbp_ipcharacter) (Math|Vector|MakeVector 0.0 0.0 1e+01))) "AlwaysSpawn" "MultiplyWithRoot" 0 0))
  (Transformation|AttachComponentToComponent _returnvalue (Variables|/Game/Data/BP_IPCharacter.BP_IPCharacter_C|GetCardAnchor _asbp_ipcharacter) "None" "SnapToTarget" "SnapToTarget" "KeepWorld" true))

(event EventTick
  (params (DeltaSeconds :type Float%20%28single-precision%29)))

(fn ConstructionScript)